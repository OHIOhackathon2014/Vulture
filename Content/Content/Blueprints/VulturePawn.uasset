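; Vulture enemy pawn with a destructible component that spawns an explosion effect at the hit point when fractured.
; Tick compares the camera's forward vector with the pawn's normalized world location, not a camera-relative direction, against a 45-degree threshold.
; Wider angles lead to downward movement, narrower ones to random impulses or movement toward the player, behind Gates that are only toggled, never entered.
; A fire effect branch is unconnected.
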(event OnComponentFracture(Destructible1)
  (params (HitPoint :type Vector%20%28by%20ref%29 :default "0, 0, 0") (HitDirection :type Vector%20%28by%20ref%29 :default "0, 0, 0"))
  (bind _returnvalue (AddComponent|AddParticleSystemComponent true (Math|Conversions|ToTransform(Vector) HitPoint)))
  (Effects|SpawnEmitterAttached "/Game/Particles/P_Explosion.P_Explosion" _returnvalue "None" "0, 0, 0" "0, 0, 0" "KeepRelativeOffset"))

(event EventTick
  (params (DeltaSeconds :type Float%20%28single-precision%29))
  (bind _returnvalue (Transformation|GetActorLocation))
  (bind _returnvalue_2 (Math|Random|RandomIntegerinRange 0 1000))
  (bind _returnvalue_3 (Math|Conversions|ToFloat(Integer) _returnvalue_2))
  (Math|Float|CompareFloat (Math|Float|Absolute(Float) (Class|KismetMathLibrary|DegAcos (Math|Vector|DotProduct (Math|Vector|Normalize _returnvalue) (Math|Vector|Normalize (Math|Rotator|GetRotationXVector (Camera|GetCameraRotation (Game|GetPlayerCameraManager 0))))))) 45.0
    (:>
      (Utilities|FlowControl|Gate false ; enters at Toggle
        (:Exit
          (Pawn|Input|AddMovementInput "0, 0,-1.000000" 1.0 true))))
    (:<
      (Utilities|FlowControl|Gate true ; enters at Toggle
        (:Exit
          (if (Math|Random|RandomBool)
            (Physics|AddImpulse (Math|Vector|MakeVector _returnvalue_3 _returnvalue_3 _returnvalue_3) false)
            (else
              (Pawn|Input|AddMovementInput (Math|Vector|Normalize (- (Transformation|GetActorLocation (Game|Player|GetPlayerPawn 0)) _returnvalue)) 1e+02 false))))))))

(fn ConstructionScript)